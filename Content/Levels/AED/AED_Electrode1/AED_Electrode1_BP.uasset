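; AED electrode 1 patch actor that snaps onto its target spot on the chest of BP_Yuri.
; BeginPlay caches the Yuri actors, and it and Tick run a collision check between the patch and the first Yuri's Electrode1 transform.
; On collision, the patch detaches, spawns a scaled-down, non-ticking Electrode1_Wrap_BP as the chest-fitted (morph target) replacement, and destroys itself.
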(event `self.ReceiveTick`
  (params (DeltaSeconds :type "Float (single-precision)"))
  (bind _returnvalue (`SceneComponent.K2_GetComponentToWorld` (`self.AED_Electrode1`)))
  (bind _returnvalue_2 (`SceneComponent.K2_GetComponentToWorld` (`/Game/MetaHumans/Yuri/BP_Yuri.Electrode1` (`|GetArrayItem` (stale `self.ReceiveBeginPlay` _outactors)))))
  ;[1 1 1] check collision for patch
  (if (== _returnvalue_2 _returnvalue) :!label _label
    _
    (elif (not (stale _collided))
      (bind (_position _collided) (`PatchesCol.CheckCollision` _returnvalue _returnvalue_2))
      (if _collided
        ;[1 1 1] respawn patch on right position on chest with morph targets
        (`self.K2_DetachFromActor` "KeepRelative")
        (bind _returnvalue_3 (`|SpawnActorFromClass` "/Game/Levels/AED/AED_Electrode1/Electrode1/Electrode1_Wrap_BP.Electrode1_Wrap_BP_C" (`self.transform`) "AlwaysSpawn" "MultiplyWithRoot" null null))
        (`self.SetActorTickEnabled` _returnvalue_3 false)
        (`self.SetActorScale3D` _returnvalue_3 (0.015 0.015 0.015))
        (`self.K2_DestroyActor`)))))

(event `self.ReceiveBeginPlay`
  (bind _outactors (`GameplayStatics.GetAllActorsOfClass` "/Game/MetaHumans/Yuri/BP_Yuri.BP_Yuri_C"))
  (goto _label))

(fn `UserConstructionScript`)